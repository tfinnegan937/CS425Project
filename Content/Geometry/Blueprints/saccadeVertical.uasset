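; Actor for a vertical saccade eye test that moves a ball stimulus, hidden at BeginPlay.
; StartTest attaches and shows the ball, then activates the root, whose activation event loops latent moves up by MoveDistance and a near-instant return until TestCount reaches ten.
; StopTest only hides the ball, leaving the loop and counter untouched.
; Tick queries both pupil positions without using the results.
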(event `self.ReceiveBeginPlay`
  (`SceneComponent.SetVisibility` (`self.ball`) false false))

(event `self.ReceiveTick`
  (params (DeltaSeconds :type "Float (single-precision)"))
  (`SRanipalEye_FunctionLibrary.GetPupilPosition` "LEFT")
  (`SRanipalEye_FunctionLibrary.GetPupilPosition` "RIGHT"))

(event `self.DefaultSceneRoot.OnComponentActivated`
  (params (Component :type "ActorComponent Object Reference") (bReset :type Boolean))
  (bind _ball (`self.ball`))
  (bind _movedistance (`self.moveDistance`))
  (bind _ball_2 (`self.ball`))
  (bind (_relativelocation_x _relativelocation_y _relativelocation_z) (`KismetMathLibrary.BreakVector` (`SceneComponent.RelativeLocation` _ball)))
  (bind (_relativelocation_x_2 _relativelocation_y_2 _relativelocation_z_2) (`KismetMathLibrary.BreakVector` (`SceneComponent.RelativeLocation` _ball_2)))
  (`KismetSystemLibrary.MoveComponentTo` _ball (`KismetMathLibrary.MakeVector` _relativelocation_x _relativelocation_y (+ _relativelocation_z _movedistance)) (struct) false false 0.6 :!label _label)
  (`KismetSystemLibrary.MoveComponentTo` _ball_2 (`KismetMathLibrary.MakeVector` _relativelocation_x_2 _relativelocation_y_2 (- _relativelocation_z_2 _movedistance)) (struct) false false 0.01)
  (set `self.testCount` (+ (`self.testCount`) 1))
  (if (< (`self.testCount`) 10)
    (goto _label)))

(event `self.ball.OnComponentActivated`
  (params (Component :type "ActorComponent Object Reference") (bReset :type Boolean)))

(fn `startTest`
  (bind _defaultsceneroot (`self.DefaultSceneRoot`))
  (`SceneComponent.K2_AttachToComponent` (`self.ball`) _defaultsceneroot "None" "KeepRelative" "KeepRelative" "KeepRelative" true)
  (`SceneComponent.SetVisibility` (`self.ball`) true false)
  (`ActorComponent.Activate` _defaultsceneroot false))

(fn `StopTest`
  (`SceneComponent.SetVisibility` (`self.ball`) false false))

(fn `UserConstructionScript`)