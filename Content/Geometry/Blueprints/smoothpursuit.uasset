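; Smooth pursuit eye test actor that shows a moving Ball as a visual target.
; StartTest reveals the ball and activates the root component, whose activation event chains timed MoveComponentTo sweeps along Y, then Z, out and back through center.
; TestCount repeats the pattern four times before hiding the ball; StopTest only hides it, without halting movement.
; Tick polls both pupil positions but leaves the results unused.
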(event `self.ReceiveBeginPlay`
  (`SceneComponent.SetVisibility` (`self.ball`) false false))

(event `self.DefaultSceneRoot.OnComponentActivated`
  (params (Component :type "ActorComponent Object Reference") (bReset :type Boolean))
  (bind _ball (`self.ball`))
  (bind _ball_2 (`self.ball`))
  (bind _ball_3 (`self.ball`))
  (bind _ball_4 (`self.ball`))
  (bind _ball_5 (`self.ball`))
  (bind _ball_6 (`self.ball`))
  (bind _returnvalue (< (`self.testCount`) 4))
  (bind (_relativelocation_x _relativelocation_y _relativelocation_z) (`KismetMathLibrary.BreakVector` (`SceneComponent.RelativeLocation` _ball)))
  (bind (_relativelocation_x_2 _relativelocation_y_2 _relativelocation_z_2) (`KismetMathLibrary.BreakVector` (`SceneComponent.RelativeLocation` _ball_3)))
  (bind (_relativelocation_x_3 _relativelocation_y_3 _relativelocation_z_3) (`KismetMathLibrary.BreakVector` (`SceneComponent.RelativeLocation` _ball_4)))
  (bind (_relativelocation_x_4 _relativelocation_y_4 _relativelocation_z_4) (`KismetMathLibrary.BreakVector` (`SceneComponent.RelativeLocation` _ball_2)))
  (bind (_relativelocation_x_5 _relativelocation_y_5 _relativelocation_z_5) (`KismetMathLibrary.BreakVector` (`SceneComponent.RelativeLocation` _ball_5)))
  (bind (_relativelocation_x_6 _relativelocation_y_6 _relativelocation_z_6) (`KismetMathLibrary.BreakVector` (`SceneComponent.RelativeLocation` _ball_6)))
  (`KismetSystemLibrary.MoveComponentTo` _ball_4 (`KismetMathLibrary.MakeVector` _relativelocation_x_3 (+ _relativelocation_y_3 (`self.moveDistance`)) _relativelocation_z_3) (struct) false false 2.0 :!label _label)
  (`KismetSystemLibrary.MoveComponentTo` (`self.ball`) (`KismetMathLibrary.MakeVector` _relativelocation_x_3 (- _relativelocation_y_3 (`self.moveDistance`)) _relativelocation_z_3) (struct) false false 2.0)
  (`KismetSystemLibrary.MoveComponentTo` _ball_3 (`KismetMathLibrary.MakeVector` _relativelocation_x_2 (- _relativelocation_y_2 (`self.moveDistance`)) _relativelocation_z_2) (struct) false false 2.0)
  (`KismetSystemLibrary.MoveComponentTo` _ball_5 (`KismetMathLibrary.MakeVector` _relativelocation_x_5 (+ _relativelocation_y_5 (`self.moveDistance`)) _relativelocation_z_5) (struct) false false 2.0)
  (`KismetSystemLibrary.MoveComponentTo` _ball (`KismetMathLibrary.MakeVector` _relativelocation_x _relativelocation_y (+ _relativelocation_z (`self.moveDistance`))) (struct) false false 2.0)
  (`KismetSystemLibrary.MoveComponentTo` (`self.ball`) (`KismetMathLibrary.MakeVector` _relativelocation_x _relativelocation_y (- _relativelocation_z (`self.moveDistance`))) (struct) false false 2.0)
  (`KismetSystemLibrary.MoveComponentTo` _ball_6 (`KismetMathLibrary.MakeVector` _relativelocation_x_6 _relativelocation_y_6 (- _relativelocation_z_6 (`self.moveDistance`))) (struct) false false 2.0)
  (`KismetSystemLibrary.MoveComponentTo` _ball_2 (`KismetMathLibrary.MakeVector` _relativelocation_x_4 _relativelocation_y_4 (+ _relativelocation_z_4 (`self.moveDistance`))) (struct) false false 2.0)
  (set `self.testCount` (+ (`self.testCount`) 1))
  (if _returnvalue
    (goto _label)
    (else
      (`SceneComponent.SetVisibility` (`self.ball`) _returnvalue false))))

(event `self.ReceiveTick`
  (params (DeltaSeconds :type "Float (single-precision)"))
  (`SRanipalEye_FunctionLibrary.GetPupilPosition` "RIGHT")
  (`SRanipalEye_FunctionLibrary.GetPupilPosition` "LEFT"))

(fn `StartTest`
  (bind _defaultsceneroot (`self.DefaultSceneRoot`))
  (`SceneComponent.K2_AttachToComponent` (`self.ball`) _defaultsceneroot "None" "KeepRelative" "KeepRelative" "KeepRelative" true)
  (`SceneComponent.SetVisibility` (`self.ball`) true false)
  (`ActorComponent.Activate` _defaultsceneroot false))

(fn `StopTest`
  (`SceneComponent.SetVisibility` (`self.ball`) false false))

(fn `UserConstructionScript`)