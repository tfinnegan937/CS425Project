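; Smooth pursuit eye-tracking test actor that moves a ball for the player to follow and samples both pupil positions while not completed.
; Once begun, chained MoveComponentTo calls sweep the ball horizontally and vertically around its start for two cycles, then hide and reset it.
; The UI controller then gathers symptom ratings, and its FogginessDone event triggers saving them and marks the test complete.
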(event `self.ReceiveTick`
  (params (DeltaSeconds :type "Float (single-precision)"))
  (if (not (`self.isCompleted`))
    (`SRanipalEye_FunctionLibrary.GetPupilPosition` "LEFT")
    (`SRanipalEye_FunctionLibrary.GetPupilPosition` "RIGHT")))

(event `self.ReceiveBeginPlay`
  (bind _ball (`self.ball`))
  (bind (_relativelocation_x _relativelocation_y _relativelocation_z) (`KismetMathLibrary.BreakVector` (`SceneComponent.RelativeLocation` _ball)))
  (`SceneComponent.SetVisibility` _ball false false)
  (set `self.StartingLocation` (`KismetMathLibrary.MakeVector` _relativelocation_x _relativelocation_y _relativelocation_z)))

(event `self.StartTest`
  (set `self.isCompleted` false)
  (`/Game/TestBlueprintClasses/AUIControllerBP.SmoothPursuitStart_Event` (`self.UIController`)))

(event `TestBegin_Event`
  (bind _uicontroller (`self.UIController`))
  (bind _ball (`self.ball`))
  (bind _ball_2 (`self.ball`))
  (bind _ball_3 (`self.ball`))
  (bind _testcycles (`self.testCycles`))
  (bind _uicontroller_2 (`self.UIcontroller`))
  (bind _ball_4 (`self.ball`))
  (bind _ball_5 (`self.ball`))
  (bind _ball_6 (`self.ball`))
  (bind (_relativelocation_x _relativelocation_y _relativelocation_z) (`KismetMathLibrary.BreakVector` (`SceneComponent.RelativeLocation` _ball_2)))
  (bind (_relativelocation_x_2 _relativelocation_y_2 _relativelocation_z_2) (`KismetMathLibrary.BreakVector` (`SceneComponent.RelativeLocation` _ball_3)))
  (bind (_relativelocation_x_3 _relativelocation_y_3 _relativelocation_z_3) (`KismetMathLibrary.BreakVector` (`SceneComponent.RelativeLocation` _ball)))
  (bind _smoothpursuit (`/Game/TestBlueprintClasses/AUIControllerBP.SmoothPursuit` (`self.UIController`)))
  (bind (_relativelocation_x_4 _relativelocation_y_4 _relativelocation_z_4) (`KismetMathLibrary.BreakVector` (`SceneComponent.RelativeLocation` _ball_4)))
  (bind (_relativelocation_x_5 _relativelocation_y_5 _relativelocation_z_5) (`KismetMathLibrary.BreakVector` (`SceneComponent.RelativeLocation` _ball_5)))
  (bind (_relativelocation_x_6 _relativelocation_y_6 _relativelocation_z_6) (`KismetMathLibrary.BreakVector` (`SceneComponent.RelativeLocation` _ball_6)))
  (`SceneComponent.K2_AddLocalOffset` (`/Game/TestBlueprintClasses/AUIControllerBP.SmoothPursuit` _uicontroller) (`/Game/TestBlueprintClasses/AUIControllerBP.return offset` _uicontroller) false true)
  (`ActorComponent.SetActive` _smoothpursuit false false)
  (`PrimitiveComponent.SetCollisionEnabled` _smoothpursuit "NoCollision")
  (`KismetSystemLibrary.PrintString` "Test Started")
  (set `self.isCompleted` false)
  (`SceneComponent.SetVisibility` _ball_3 true false)
  (`KismetSystemLibrary.MoveComponentTo` _ball_3 (`KismetMathLibrary.MakeVector` _relativelocation_x_2 (+ _relativelocation_y_2 (`self.moveDistance`)) _relativelocation_z_2) (struct) false false 2.0 :!label _label)
  (`KismetSystemLibrary.MoveComponentTo` (`self.ball`) (`KismetMathLibrary.MakeVector` _relativelocation_x_2 (- _relativelocation_y_2 (`self.moveDistance`)) _relativelocation_z_2) (struct) false false 2.0)
  (`KismetSystemLibrary.MoveComponentTo` _ball_2 (`KismetMathLibrary.MakeVector` _relativelocation_x (- _relativelocation_y (`self.moveDistance`)) _relativelocation_z) (struct) false false 2.0)
  (`KismetSystemLibrary.MoveComponentTo` _ball_4 (`KismetMathLibrary.MakeVector` _relativelocation_x_4 (+ _relativelocation_y_4 (`self.moveDistance`)) _relativelocation_z_4) (struct) false false 2.0)
  (`KismetSystemLibrary.MoveComponentTo` _ball_5 (`KismetMathLibrary.MakeVector` _relativelocation_x_5 _relativelocation_y_5 (+ _relativelocation_z_5 (`self.moveDistance`))) (struct) false false 2.0)
  (`KismetSystemLibrary.MoveComponentTo` (`self.ball`) (`KismetMathLibrary.MakeVector` _relativelocation_x_5 _relativelocation_y_5 (- _relativelocation_z_5 (`self.moveDistance`))) (struct) false false 2.0)
  (`KismetSystemLibrary.MoveComponentTo` _ball_6 (`KismetMathLibrary.MakeVector` _relativelocation_x_6 _relativelocation_y_6 (- _relativelocation_z_6 (`self.moveDistance`))) (struct) false false 2.0)
  (`KismetSystemLibrary.MoveComponentTo` _ball (`KismetMathLibrary.MakeVector` _relativelocation_x_3 _relativelocation_y_3 (+ _relativelocation_z_3 (`self.moveDistance`))) (struct) false false 2.0)
  (set `self.testCycles` (+ _testcycles 1))
  (if (< _testcycles 2)
    (goto _label)
    (else
      (`SceneComponent.SetVisibility` (`self.ball`) false false)
      (`KismetSystemLibrary.MoveComponentTo` (`self.ball`) (`self.StartingLocation`) (struct) false false 0.01)
      (set `/Game/TestBlueprintClasses/AUIControllerBP.OutsideTest` true (`self.UIController`))
      (`/Game/TestBlueprintClasses/AUIControllerBP.getSymptomData` _uicontroller_2)
      (add `/Game/TestBlueprintClasses/AUIControllerBP.FogginessDone` _uicontroller_2 (delegate `symptomsDone_Event`)))))

(event `symptomsDone_Event`
  (bind _uicontroller (`self.UIcontroller`))
  (`self.SaveSymptomData` (`/Game/TestBlueprintClasses/AUIControllerBP.HeadacheVal` _uicontroller) (`/Game/TestBlueprintClasses/AUIControllerBP.DizzinessVal` _uicontroller) (`/Game/TestBlueprintClasses/AUIControllerBP.NauseaVal` _uicontroller) (`/Game/TestBlueprintClasses/AUIControllerBP.FogginessVal` _uicontroller))
  (set `self.isCompleted` true)
  (clear `/Game/TestBlueprintClasses/AUIControllerBP.FogginessDone` (`self.UIController`)))

(event `self.StopTest`
  (bind _ball (`self.ball`))
  (`SceneComponent.SetVisibility` _ball false false)
  (set `self.isCompleted` true)
  (`KismetSystemLibrary.MoveComponentTo` _ball (`self.StartingLocation`) (struct) false false 0.01))

(fn `UserConstructionScript`)