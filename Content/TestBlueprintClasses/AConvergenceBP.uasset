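; AConvergenceBP is a VR eye-convergence test actor that shows a sphere and records gaze and controller-measured distances.
; While a test runs, Tick saves gaze, sphere and head data every frame.
; setDistance input captures motion controller positions; after repeated releases, one doubled initial-to-final distance is saved as all three results.
; It then hides the sphere, collects symptom ratings through UIcontroller, saves them and ends the test.
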(event `self.ReceiveBeginPlay`
  (set `self.isCompleted` true)
  (`SceneComponent.SetVisibility` (`self.Sphere`) false false)
  (`self.EnableInput` (`GameplayStatics.GetPlayerController` 0)))

(event `self.ReceiveTick`
  (params (DeltaSeconds :type "Float (single-precision)"))
  (bind _returnvalue_location (`KismetMathLibrary.BreakTransform` (`self.GetTransform`)))
  (bind _hmd (`self.HMD`))
  (bind _returnvalue_location_2 (`KismetMathLibrary.BreakTransform` (`SceneComponent.GetRelativeTransform` (`self.Sphere`))))
  (bind _returnvalue_location_3 (`KismetMathLibrary.BreakTransform` (`self.GetTransform` _hmd)))
  (bind (_returnvalue_location_4 _returnvalue_rotation) (`KismetMathLibrary.BreakTransform` (`SceneComponent.GetRelativeTransform` (`self.GetComponentByClass` _hmd "/Script/Engine.CameraComponent"))))
  (bind (_returnvalue_location_5 _returnvalue_rotation_2) (`KismetMathLibrary.BreakTransform` (`SceneComponent.GetRelativeTransform` (`|GetArrayItem` (`self.GetComponentsByTag` _hmd "/Script/Engine.SceneComponent" "Root")))))
  (if (not (`self.isCompleted`))
    (bind _outgazedata (`EyeTrackerFunctionLibrary.GetGazeData`))
    (bind _outgazedata_2 (`EyeTrackerFunctionLibrary.GetStereoGazeData`))
    (bind _output_get (set `self.TimeSinceStart` (+ (`self.TimeSinceStart`) 1.0)))
    (`self.SaveEyeFrameData` _output_get 5 _outgazedata _outgazedata_2 _returnvalue_location_2 (+ _returnvalue_location_2 _returnvalue_location) (+ (+ _returnvalue_location_3 _returnvalue_location_5) _returnvalue_location_4) (+ (`KismetMathLibrary.Conv_RotatorToVector` _returnvalue_rotation_2) (`KismetMathLibrary.Conv_RotatorToVector` _returnvalue_rotation)))
    (else
      (set `self.TimeSinceStart` DeltaSeconds))))

(event `InputAction|setDistance`
  (params (Key :type "Key Structure"))
  (bind _uicontroller (`self.UIcontroller`))
  (bind _testactive (`self.testActive`))
  (:`Pressed`
    (if _testactive
      (if (`self.set initial value`)
        (set `self.InitialPosition` (`SceneComponent.K2_GetComponentLocation` (`self.MotionController`)))
        (set `self.setfocaldistance` true)
        (set `self.set initial value` false)
        (elif (`self.setfocaldistance`)
          (switch `int` 0
            (:`0`
              (bind _output_get (set `self.final position` (`SceneComponent.K2_GetComponentLocation` (`self.MotionController`)))))
            (:`1`
              (bind _output_get_2 (set `self.final position` (`SceneComponent.K2_GetComponentLocation` (`self.MotionController`)))))
            (:`2`
              (bind _output_get_3 (set `self.final position` (`SceneComponent.K2_GetComponentLocation` (`self.MotionController`))))))))))
  (:`Released`
    (if _testactive
      (if (`self.set initial value`)
        (set `self.set initial value` false)
        (set `self.setfocaldistance` true)
        (else
          (bind _output_get_4 (set `self.testcount` (+ (`self.testcount`) 1)))
          (if (> _output_get_4 2)
            (`self.SaveConvergenceData` (* (`KismetMathLibrary.VSize` (- _output_get (`self.InitialPosition`))) 2.0) (* (`KismetMathLibrary.VSize` (- _output_get_2 (`self.InitialPosition`))) 2.0) (* (`KismetMathLibrary.VSize` (- _output_get_3 (`self.InitialPosition`))) 2.0))
            (`SceneComponent.SetVisibility` (`self.Sphere`) false false)
            (set `/Game/TestBlueprintClasses/AUIControllerBP.OutsideTest` true (`self.UIcontroller`))
            (`/Game/TestBlueprintClasses/AUIControllerBP.getSymptomData` _uicontroller)
            (add `/Game/TestBlueprintClasses/AUIControllerBP.FogginessDone` _uicontroller (delegate `SymptomsDone_Event`))))))))

(event `SymptomsDone_Event`
  (bind _uicontroller (`self.UIcontroller`))
  (`self.SaveSymptomData` (`/Game/TestBlueprintClasses/AUIControllerBP.HeadacheVal` _uicontroller) (`/Game/TestBlueprintClasses/AUIControllerBP.DizzinessVal` _uicontroller) (`/Game/TestBlueprintClasses/AUIControllerBP.NauseaVal` _uicontroller) (`/Game/TestBlueprintClasses/AUIControllerBP.FogginessVal` _uicontroller))
  (set `self.testActive` false)
  (clear `/Game/TestBlueprintClasses/AUIControllerBP.FogginessDone` _uicontroller)
  (set `self.isCompleted` true))

(event `self.StartTest`
  (set `self.isCompleted` false)
  (`/Game/TestBlueprintClasses/AUIControllerBP.ConvergenceStart_Event` (`self.UIcontroller`)))

(event `beginTest_Event`
  (bind _uicontroller (`self.UIController`))
  (bind _convergence (`/Game/TestBlueprintClasses/AUIControllerBP.Convergence` (`self.UIcontroller`)))
  (`SceneComponent.K2_AddLocalOffset` (`/Game/TestBlueprintClasses/AUIControllerBP.Convergence` _uicontroller) (`/Game/TestBlueprintClasses/AUIControllerBP.return offset` _uicontroller) false true)
  (set `self.testActive` true)
  (`PrimitiveComponent.SetCollisionEnabled` _convergence "NoCollision")
  (`SceneComponent.SetVisibility` (`self.Sphere`) true false)
  (`ActorComponent.SetActive` _convergence false false))

(fn `UserConstructionScript`)