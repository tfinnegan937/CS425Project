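; Horizontal saccades eye test that shows a ball moving along Y while sampling left and right pupil positions on Tick.
; StartTest loops latent MoveComponentTo calls, gliding the ball out and snapping it back until TestCount reaches ten.
; On completion it hides and resets the ball, then pulls symptom ratings from the UI controller and saves them.
; StopTest hides and resets the ball and flags completion without saving symptoms.
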(event `self.ReceiveBeginPlay`
  (bind (_relativelocation_x _relativelocation_y _relativelocation_z) (`KismetMathLibrary.BreakVector` (`SceneComponent.RelativeLocation` (`self.ball`))))
  (`SceneComponent.SetVisibility` (`self.ball`) false false)
  (set `self.StartingLocation` (`KismetMathLibrary.MakeVector` _relativelocation_x _relativelocation_y _relativelocation_z)))

(event `self.ReceiveTick`
  (params (DeltaSeconds :type "Float (single-precision)"))
  (if (not (`self.isCompleted`))
    (`SRanipalEye_FunctionLibrary.GetPupilPosition` "LEFT")
    (`SRanipalEye_FunctionLibrary.GetPupilPosition` "RIGHT")))

(event `self.StartTest`
  (bind _movedistance (`self.moveDistance`))
  (bind _uicontroller (`self.UIcontroller`))
  (bind _ball (`self.ball`))
  (bind _ball_2 (`self.ball`))
  (bind (_relativelocation_x _relativelocation_y _relativelocation_z) (`KismetMathLibrary.BreakVector` (`SceneComponent.RelativeLocation` _ball_2)))
  (bind (_relativelocation_x_2 _relativelocation_y_2 _relativelocation_z_2) (`KismetMathLibrary.BreakVector` (`SceneComponent.RelativeLocation` _ball)))
  (`SceneComponent.SetVisibility` (`self.ball`) true false)
  (set `self.isCompleted` false)
  (`KismetSystemLibrary.MoveComponentTo` _ball (`KismetMathLibrary.MakeVector` _relativelocation_x_2 (+ _relativelocation_y_2 _movedistance) _relativelocation_z_2) (struct) false false 0.6 :!label _label)
  (`KismetSystemLibrary.MoveComponentTo` _ball_2 (`KismetMathLibrary.MakeVector` _relativelocation_x (- _relativelocation_y _movedistance) _relativelocation_z) (struct) false false 0.01)
  (set `self.testCount` (+ (`self.testCount`) 1))
  (if (< (`self.testCount`) 10)
    (goto _label)
    (else
      (`SceneComponent.SetVisibility` (`self.ball`) false false)
      (set `self.isCompleted` true)
      (`KismetSystemLibrary.MoveComponentTo` (`self.ball`) (`self.StartingLocation`) (struct) false false 0.0)
      (set `/Game/TestBlueprintClasses/AUIControllerBP.OutsideTest` true (`self.UIController`))
      (`/Game/TestBlueprintClasses/AUIControllerBP.getSymptomData` _uicontroller)
      (`self.SaveSymptomData` (`/Game/TestBlueprintClasses/AUIControllerBP.HeadacheVal` _uicontroller) (`/Game/TestBlueprintClasses/AUIControllerBP.DizzinessVal` _uicontroller) (`/Game/TestBlueprintClasses/AUIControllerBP.NauseaVal` _uicontroller) (`/Game/TestBlueprintClasses/AUIControllerBP.FogginessVal` _uicontroller)))))

(event `self.StopTest`
  (`SceneComponent.SetVisibility` (`self.ball`) false false)
  (set `self.isCompleted` true)
  (`KismetSystemLibrary.MoveComponentTo` (`self.ball`) (`self.StartingLocation`) (struct) false false 0.0))

(fn `UserConstructionScript`)