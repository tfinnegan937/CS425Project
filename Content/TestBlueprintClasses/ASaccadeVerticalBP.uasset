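; Vertical saccade eye-test actor that moves a ball stimulus, samples pupil positions and records symptoms.
; StartTest shows the UIController prompt; continuing hides the ball's idle state by revealing it, then loops ten timed upward moves with near-instant returns using latent MoveComponentTo.
; Tick reads both pupils until completion.
; Afterwards the UI gathers headache, dizziness, nausea and fogginess ratings, which are saved through a bound completion event; StopTest aborts and resets.
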(event `self.ReceiveBeginPlay`
  (bind _ball (`self.ball`))
  (bind (_relativelocation_x _relativelocation_y _relativelocation_z) (`KismetMathLibrary.BreakVector` (`SceneComponent.RelativeLocation` _ball)))
  (`SceneComponent.SetVisibility` _ball false false)
  (set `self.StartingLocation` (`KismetMathLibrary.MakeVector` _relativelocation_x _relativelocation_y _relativelocation_z)))

(event `continue selected_Event`
  (bind _uicontroller (`self.UIController`))
  (bind _movedistance (`self.moveDistance`))
  (bind _ball (`self.ball`))
  (bind _ball_2 (`self.ball`))
  (bind _saccadevertical (`/Game/TestBlueprintClasses/AUIControllerBP.SaccadeVertical` (`self.UIController`)))
  (bind (_relativelocation_x _relativelocation_y _relativelocation_z) (`KismetMathLibrary.BreakVector` (`SceneComponent.RelativeLocation` _ball_2)))
  (bind (_relativelocation_x_2 _relativelocation_y_2 _relativelocation_z_2) (`KismetMathLibrary.BreakVector` (`SceneComponent.RelativeLocation` _ball)))
  (`SceneComponent.K2_AddLocalOffset` (`/Game/TestBlueprintClasses/AUIControllerBP.SaccadeVertical` _uicontroller) (`/Game/TestBlueprintClasses/AUIControllerBP.return offset` _uicontroller) false true)
  (`ActorComponent.SetActive` _saccadevertical false false)
  (`PrimitiveComponent.SetCollisionEnabled` _saccadevertical "NoCollision")
  (`SceneComponent.SetVisibility` _ball true false)
  (set `self.isCompleted` false)
  (`KismetSystemLibrary.MoveComponentTo` _ball (`KismetMathLibrary.MakeVector` _relativelocation_x_2 _relativelocation_y_2 (+ _relativelocation_z_2 _movedistance)) (struct) false false 0.6 :!label _label)
  (`KismetSystemLibrary.MoveComponentTo` _ball_2 (`KismetMathLibrary.MakeVector` _relativelocation_x _relativelocation_y (- _relativelocation_z _movedistance)) (struct) false false 0.01)
  (set `self.testCount` (+ (`self.testCount`) 1))
  (if (< (`self.testCount`) 10)
    (goto _label)
    (else
      (`SceneComponent.SetVisibility` (`self.ball`) false false)
      (`KismetSystemLibrary.MoveComponentTo` (`self.ball`) (`self.StartingLocation`) (struct) false false 0.0)
      (set `/Game/TestBlueprintClasses/AUIControllerBP.OutsideTest` true (`self.UIController`))
      (`/Game/TestBlueprintClasses/AUIControllerBP.getSymptomData` (`self.UIcontroller`)))))

(event `self.ReceiveTick`
  (params (DeltaSeconds :type "Float (single-precision)"))
  (if (not (`self.isCompleted`))
    (`SRanipalEye_FunctionLibrary.GetPupilPosition` "LEFT")
    (`SRanipalEye_FunctionLibrary.GetPupilPosition` "RIGHT")))

(event `self.StartTest`
  (add `/Game/TestBlueprintClasses/AUIControllerBP.FogginessDone` (`self.UIcontroller`) (delegate `symptomsDone_Event`))
  (set `self.isCompleted` false)
  (`SceneComponent.SetVisibility` (`/Game/TestBlueprintClasses/AUIControllerBP.SaccadeVertical` (`self.UIController`)) true false))

(event `symptomsDone_Event`
  (bind _uicontroller (`self.UIcontroller`))
  (`self.SaveSymptomData` (`/Game/TestBlueprintClasses/AUIControllerBP.HeadacheVal` _uicontroller) (`/Game/TestBlueprintClasses/AUIControllerBP.DizzinessVal` _uicontroller) (`/Game/TestBlueprintClasses/AUIControllerBP.NauseaVal` _uicontroller) (`/Game/TestBlueprintClasses/AUIControllerBP.FogginessVal` _uicontroller))
  (set `self.isCompleted` true)
  (remove `/Game/TestBlueprintClasses/AUIControllerBP.FogginessDone` (`self.UIController`) (delegate `symptomsDone_Event`)))

(event `self.StopTest`
  (bind _ball (`self.ball`))
  (`SceneComponent.SetVisibility` _ball false false)
  (set `self.isCompleted` true)
  (`KismetSystemLibrary.MoveComponentTo` _ball (`self.StartingLocation`) (struct) false false 0.0))

(fn `UserConstructionScript`)