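; Vertical VOR (vestibulo-ocular reflex) test actor that runs a metronome-paced trial, then records symptom scores.
; StartTest hands off to the UI controller; TestBegin_Event disables the vertical VOR start element, shows the sphere and loops metronome clicks through a Delay.
; After the last click, it hides the sphere, gathers symptom ratings through the UI controller, saves them and flags completion.
; Tick polls both pupil positions; StopTest ends early without saving.
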(event `self.ReceiveBeginPlay`
  (`SceneComponent.SetVisibility` (`self.Sphere`) false false))

(event `self.ReceiveTick`
  (params (DeltaSeconds :type "Float (single-precision)"))
  (`SRanipalEye_FunctionLibrary.GetPupilPosition` "LEFT")
  (`SRanipalEye_FunctionLibrary.GetPupilPosition` "RIGHT"))

(event `self.StartTest`
  (set `self.isCompleted` false)
  (`/Game/TestBlueprintClasses/AUIControllerBP.VORVerticalStart_Event` (`self.UIController`)))

(event `Symptom_Event`
  (bind _uicontroller (`self.UIcontroller`))
  (`self.SaveSymptomData` (`/Game/TestBlueprintClasses/AUIControllerBP.HeadacheVal` _uicontroller) (`/Game/TestBlueprintClasses/AUIControllerBP.DizzinessVal` _uicontroller) (`/Game/TestBlueprintClasses/AUIControllerBP.NauseaVal` _uicontroller) (`/Game/TestBlueprintClasses/AUIControllerBP.FogginessVal` _uicontroller))
  (set `self.isCompleted` true)
  (clear `/Game/TestBlueprintClasses/AUIControllerBP.FogginessDone` (`self.UIController`)))

(event `self.StopTest`
  (`SceneComponent.SetVisibility` (`self.Sphere`) false false)
  (set `self.isCompleted` true))

(event `TestBegin_Event`
  (bind _uicontroller (`self.UIController`))
  (bind _cycle_num (`self.cycle num`))
  (bind _uicontroller_2 (`self.UIcontroller`))
  (bind _vorvertical (`/Game/TestBlueprintClasses/AUIControllerBP.VORVertical` (`self.UIController`)))
  (`SceneComponent.K2_AddLocalOffset` (`/Game/TestBlueprintClasses/AUIControllerBP.VORVertical` _uicontroller) (`/Game/TestBlueprintClasses/AUIControllerBP.return offset` _uicontroller) false true)
  (`ActorComponent.SetActive` _vorvertical false false)
  (`PrimitiveComponent.SetCollisionEnabled` _vorvertical "NoCollision")
  (`SceneComponent.SetVisibility` (`self.Sphere`) true false)
  (`GameplayStatics.PlaySound2D` "/Game/StarterContent/Audio/metronomeSound.metronomeSound" 1.0 1.0 0.0 null null :!label _label)
  (set `self.cycle num` (+ _cycle_num 1))
  (`KismetSystemLibrary.Delay` 0.333333)
  (if (< _cycle_num 10)
    (goto _label)
    (else
      (`SceneComponent.SetVisibility` (`self.Sphere`) false false)
      (set `/Game/TestBlueprintClasses/AUIControllerBP.OutsideTest` true (`self.UIController`))
      (add `/Game/TestBlueprintClasses/AUIControllerBP.FogginessDone` _uicontroller_2 (delegate `Symptom_Event`))
      (`/Game/TestBlueprintClasses/AUIControllerBP.getSymptomData` _uicontroller_2))))

(fn `UserConstructionScript`)