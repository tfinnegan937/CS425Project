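; Controller actor for the UI panels of a vestibular and ocular-motor screening test, covering symptom questions and test start screens.
; StartTest reveals Nausea, then each Done event uses WidgetDone and location offsets to swap in Headache, Fogginess and Dizziness.
; The final step saves the four values as baseline symptom data and sets IsCompleted, unless OutsideTest is set.
; Separate start events reveal the convergence, saccade, smooth pursuit, VOR and VMS panels.
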(event `self.ReceiveBeginPlay`
  (bind _convergence (`self.Convergence`))
  (bind _saccadevertical (`self.SaccadeVertical`))
  (bind _smoothpursuit (`self.SmoothPursuit`))
  (bind _vms (`self.VMS`))
  (bind _vorhorizontal (`self.VORHorizontal`))
  (bind _vorvertical (`self.VORVertical`))
  (bind _saccadehorizontal (`self.SaccadeHorizontal`))
  (`SceneComponent.SetVisibility` (`self.Nausea`) false false)
  (`SceneComponent.SetVisibility` (`self.Headache`) false false)
  (`SceneComponent.SetVisibility` (`self.Fogginess`) false false)
  (`SceneComponent.SetVisibility` (`self.Dizziness`) false false)
  (`SceneComponent.SetVisibility` _convergence false false)
  (`PrimitiveComponent.SetCollisionEnabled` _convergence "NoCollision")
  (`SceneComponent.SetVisibility` _saccadevertical false false)
  (`PrimitiveComponent.SetCollisionEnabled` _saccadevertical "NoCollision")
  (`SceneComponent.SetVisibility` _smoothpursuit false false)
  (`PrimitiveComponent.SetCollisionEnabled` _smoothpursuit "NoCollision")
  (`SceneComponent.SetVisibility` _vms false false)
  (`PrimitiveComponent.SetCollisionEnabled` _vms "NoCollision")
  (`SceneComponent.SetVisibility` _vorhorizontal false false)
  (`PrimitiveComponent.SetCollisionEnabled` _vorhorizontal "NoCollision")
  (`SceneComponent.SetVisibility` _vorvertical false false)
  (`PrimitiveComponent.SetCollisionEnabled` _vorvertical "NoCollision")
  (`SceneComponent.SetVisibility` _saccadehorizontal false false)
  (`PrimitiveComponent.SetCollisionEnabled` _saccadehorizontal "NoCollision"))

(event `self.StartTest`
  (`self.getSymptomData`))

(event `NauseaDone_Event`
  (bind _nausea (`self.Nausea`))
  (bind _headache (`self.Headache`))
  (`SceneComponent.K2_AddLocalOffset` _nausea (`self.return offset`) false false)
  (`self.WidgetDone` _nausea _headache)
  (`SceneComponent.K2_AddLocalOffset` _headache (`self.location offset`) false true))

(event `HeadacheDone_Event`
  (bind _fogginess (`self.Fogginess`))
  (`SceneComponent.K2_AddLocalOffset` (`self.Headache`) (`self.return offset`) false false)
  (`self.WidgetDone` (`self.Headache`) _fogginess)
  (`SceneComponent.K2_AddLocalOffset` _fogginess (`self.location offset`) false true))

(event `FogginessDone_Event`
  (bind _dizziness (`self.Dizziness`))
  (`SceneComponent.K2_AddLocalOffset` (`self.Fogginess`) (`self.return offset`) false true)
  (`self.WidgetDone` (`self.Fogginess`) _dizziness)
  (`SceneComponent.K2_AddLocalOffset` _dizziness (`self.location offset`) false true))

(event `DizzinessDone_Event`
  (bind _dizziness (`self.Dizziness`))
  (bind _dizziness_2 (`self.Dizziness`))
  (if (`self.OutsideTest`)
    (`PrimitiveComponent.SetCollisionEnabled` (`self.Dizziness`) "NoCollision")
    (`SceneComponent.SetVisibility` _dizziness false false)
    (`ActorComponent.SetActive` _dizziness false false)
    (`SceneComponent.K2_AddLocalOffset` (`self.Nausea`) (`self.return offset`) false false)
    (else
      (`PrimitiveComponent.SetCollisionEnabled` (`self.Dizziness`) "NoCollision")
      (`SceneComponent.SetVisibility` _dizziness_2 false false)
      (`ActorComponent.SetActive` _dizziness_2 false false)
      (`SceneComponent.K2_AddLocalOffset` (`self.Nausea`) (`self.return offset`) false true)
      (`self.SaveSymptomData` (`self.HeadacheVal`) (`self.DizzinessVal`) (`self.NauseaVal`) (`self.FogginessVal`) true)
      (set `self.isCompleted` true))))

(event `ConvergenceStart_Event`
  (bind _convergence (`self.Convergence`))
  (`SceneComponent.K2_AddLocalOffset` (`self.Convergence`) (`self.location offset`) false false)
  (`ActorComponent.SetActive` _convergence true false)
  (`SceneComponent.SetVisibility` _convergence true false)
  (`PrimitiveComponent.SetCollisionEnabled` _convergence "QueryOnly"))

(event `SaccadeHorizontalStart_Event`
  (bind _saccadehorizontal (`self.SaccadeHorizontal`))
  (`SceneComponent.K2_AddLocalOffset` _saccadehorizontal (`self.location offset`) false false)
  (`ActorComponent.SetActive` _saccadehorizontal true false)
  (`SceneComponent.SetVisibility` _saccadehorizontal true false)
  (`PrimitiveComponent.SetCollisionEnabled` _saccadehorizontal "QueryOnly"))

(event `SaccadeVerticalStart_Event`
  (bind _saccadevertical (`self.SaccadeVertical`))
  (`SceneComponent.K2_AddLocalOffset` _saccadevertical (`self.location offset`) false false)
  (`ActorComponent.SetActive` _saccadevertical true false)
  (`SceneComponent.SetVisibility` _saccadevertical true false)
  (`PrimitiveComponent.SetCollisionEnabled` _saccadevertical "QueryOnly"))

(event `SmoothPursuitStart_Event`
  (bind _smoothpursuit (`self.SmoothPursuit`))
  (`SceneComponent.K2_AddLocalOffset` _smoothpursuit (`self.location offset`) false false)
  (`ActorComponent.SetActive` _smoothpursuit false false)
  (`SceneComponent.SetVisibility` _smoothpursuit true false)
  (`PrimitiveComponent.SetCollisionEnabled` _smoothpursuit "QueryOnly"))

(event `VORVerticalStart_Event`
  (bind _vorvertical (`self.VORVertical`))
  (`SceneComponent.K2_AddLocalOffset` _vorvertical (`self.location offset`) false false)
  (`ActorComponent.SetActive` _vorvertical false false)
  (`SceneComponent.SetVisibility` _vorvertical true false)
  (`PrimitiveComponent.SetCollisionEnabled` _vorvertical "QueryOnly"))

(event `VORHorizontalStart_Event`
  (bind _vorhorizontal (`self.VORHorizontal`))
  (`SceneComponent.K2_AddLocalOffset` _vorhorizontal (`self.location offset`) false false)
  (`ActorComponent.SetActive` _vorhorizontal false false)
  (`SceneComponent.SetVisibility` _vorhorizontal true false)
  (`PrimitiveComponent.SetCollisionEnabled` _vorhorizontal "QueryOnly"))

(event `VMSStart_Event`
  (bind _vms (`self.VMS`))
  (`SceneComponent.K2_AddLocalOffset` _vms (`self.location offset`) false false)
  (`ActorComponent.SetActive` _vms false false)
  (`SceneComponent.SetVisibility` _vms true false)
  (`PrimitiveComponent.SetCollisionEnabled` _vms "QueryOnly"))

(fn `getSymptomData`
  (bind _nausea (`self.Nausea`))
  (`PrimitiveComponent.SetCollisionEnabled` (`self.Nausea`) "QueryOnly")
  (`SceneComponent.ToggleVisibility` _nausea false)
  (`ActorComponent.SetActive` _nausea true false)
  (if (not (`self.OutsideTest`))
    (set `self.isCompleted` false)))

(fn `UserConstructionScript`)

(fn `WidgetDone`
  (params (TestDone :type "WidgetComponent Object Reference") (TestStart :type "WidgetComponent Object Reference") (TestActor :type "CSVStreamableActor Object Reference") (TestPawn :type "CSVStreamablePawn Object Reference"))
  (`SceneComponent.K2_AddLocalOffset` TestDone (`self.return offset`) false true)
  (`ActorComponent.SetActive` TestDone false false)
  (`PrimitiveComponent.SetCollisionEnabled` TestDone "NoCollision")
  (`SceneComponent.SetVisibility` TestDone false false)
  (`SceneComponent.SetVisibility` TestStart true false)
  (`PrimitiveComponent.SetCollisionEnabled` TestStart "QueryOnly")
  (`ActorComponent.SetActive` TestStart true false)
  (if true
    _))