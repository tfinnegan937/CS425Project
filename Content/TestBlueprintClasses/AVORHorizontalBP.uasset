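; Test actor for a horizontal VOR (vestibulo-ocular reflex) check that ends with a symptom survey.
; StartTest triggers the UI intro, and TestBegin_Event shows the sphere while a delay loop plays a fixed count of metronome ticks.
; It then hides the sphere and binds to the UI's fogginess-done event to save symptom scores and mark completion.
; Tick queries both pupil positions but leaves the results unused.
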(event `self.ReceiveBeginPlay`
  (`SceneComponent.SetVisibility` (`self.Sphere`) false false))

(event `self.ReceiveTick`
  (params (DeltaSeconds :type "Float (single-precision)"))
  (`SRanipalEye_FunctionLibrary.GetPupilPosition` "LEFT")
  (`SRanipalEye_FunctionLibrary.GetPupilPosition` "RIGHT"))

(event `self.StartTest`
  (set `self.isCompleted` false)
  (`/Game/TestBlueprintClasses/AUIControllerBP.VORHorizontalStart_Event` (`self.UIController`)))

(event `Symptom_Event`
  (bind _uicontroller (`self.UIcontroller`))
  (`self.SaveSymptomData` (`/Game/TestBlueprintClasses/AUIControllerBP.HeadacheVal` _uicontroller) (`/Game/TestBlueprintClasses/AUIControllerBP.DizzinessVal` _uicontroller) (`/Game/TestBlueprintClasses/AUIControllerBP.NauseaVal` _uicontroller) (`/Game/TestBlueprintClasses/AUIControllerBP.FogginessVal` _uicontroller))
  (set `self.isCompleted` true)
  (clear `/Game/TestBlueprintClasses/AUIControllerBP.FogginessDone` (`self.UIController`)))

(event `TestBegin_Event`
  (bind _cycle_num (`self.cycle num`))
  (bind _uicontroller (`self.UIcontroller`))
  (`PrimitiveComponent.SetCollisionEnabled` (`/Game/TestBlueprintClasses/AUIControllerBP.VORHorizontal` (`self.UIController`)) "NoCollision")
  (`SceneComponent.SetVisibility` (`self.Sphere`) true false)
  (`GameplayStatics.PlaySound2D` "/Game/StarterContent/Audio/metronomeSound.metronomeSound" 1.0 1.0 0.0 null null :!label _label)
  (set `self.cycle num` (+ _cycle_num 1))
  (`KismetSystemLibrary.Delay` 0.333333)
  (if (< _cycle_num 10)
    (goto _label)
    (else
      (`SceneComponent.SetVisibility` (`self.Sphere`) false false)
      (set `/Game/TestBlueprintClasses/AUIControllerBP.OutsideTest` true (`self.UIController`))
      (`/Game/TestBlueprintClasses/AUIControllerBP.getSymptomData` _uicontroller)
      (add `/Game/TestBlueprintClasses/AUIControllerBP.FogginessDone` _uicontroller (delegate `Symptom_Event`)))))

(event `self.StopTest`
  (`SceneComponent.SetVisibility` (`self.Sphere`) false false)
  (set `self.isCompleted` true))

(fn `UserConstructionScript`)